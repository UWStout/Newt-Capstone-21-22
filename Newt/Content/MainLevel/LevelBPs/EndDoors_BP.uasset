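; End doors Blueprint that closes out the level by animating the final ruins doors when an actor overlaps it.
; It stops the ruins FMOD loop, found at BeginPlay, and two timelines slide the door meshes along Y.
; After a delay it shows a leaf transition widget, then opens the CutSceneEnding level and plays the ending animatic audio event.
; An unconnected EndScreen widget branch never runs.
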(event `self.ReceiveBeginPlay`
  (bind _returnvalue (`GameplayStatics.GetActorOfClass` "/Game/Sound_Sources/Level02_Ruins/ruins_loop_start_Blueprint.ruins_loop_start_Blueprint_C"))
  (set `self.Ruins_loop` _returnvalue))

(event `self.ReceiveActorBeginOverlap`
  (params (OtherActor :type "Actor Object Reference"))
  (`FMODBlueprintStatics.EventInstanceStop` (`/Game/Sound_Sources/Level02_Ruins/ruins_loop_start_Blueprint.fmod_event_ruins_loop` (`self.Ruins_loop`)))
  (bind (_direction _newtrack_0) (`Timeline|Timeline_0`)
    (:`Update`
      (`SceneComponent.K2_SetRelativeLocation` (`self.Ruins_FinalDoor_01_pCube140`) (`KismetMathLibrary.MakeVector` 0.0 _newtrack_0) false true)
      (bind (_direction_2 _newtrack_0_2) (`Timeline|Timeline_1`)
        (:`Update`
          (`SceneComponent.K2_SetRelativeLocation` (`self.Ruins_FinalDoor_01_pCube141`) (`KismetMathLibrary.MakeVector` 0.0 _newtrack_0_2) false true)
          (`KismetSystemLibrary.Delay` 4.0)
          (bind _returnvalue (`|CreateWidget` "/Game/UI/LeafTransitionOpenNew_2.LeafTransitionOpenNew_2_C"))
          (`UserWidget.AddToViewport` _returnvalue 0)
          (`KismetSystemLibrary.Delay` 0.75)
          (`GameplayStatics.OpenLevel` "CutSceneEnding")
          (`FMODBlueprintStatics.PlayEvent2D` "/Game/FMOD/Events/music/animatics/animatic_ending.animatic_ending"))))))

(fn `UserConstructionScript`)