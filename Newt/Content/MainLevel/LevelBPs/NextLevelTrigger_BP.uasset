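; Level-exit trigger actor that moves the game on to LVL_2_Main when any actor overlaps it.
; On BeginPlay it finds and caches the cave music loop trigger actor.
; On overlap it stops and releases that actor's FMOD music event, makes a second stop call without release, and shows the CloseDoorTransition widget.
; A short delay lets the transition play before the level opens by name.
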(event `self.ReceiveBeginPlay`
  (bind _returnvalue (`GameplayStatics.GetActorOfClass` "/Game/Sound_Sources/Level01_Caves/cave_music_loop_trigger_start_Blueprint.cave_music_loop_trigger_start_Blueprint_C"))
  (set `self.Cave_loop_music_reference` _returnvalue))

(event `self.ReceiveActorBeginOverlap`
  (params (OtherActor :type "Actor Object Reference"))
  (`FMODBlueprintStatics.EventInstanceStop` (`/Game/Sound_Sources/Level01_Caves/cave_music_loop_trigger_start_Blueprint.fmod_event_mus_cave_loop_variable` (`self.Cave_loop_music_reference`)) true)
  (`FMODBlueprintStatics.EventInstanceStop` (struct))
  (bind _returnvalue (`|CreateWidget` "/Game/UI/CloseDoorTransition.CloseDoorTransition_C"))
  (`UserWidget.AddToViewport` _returnvalue 0)
  (`KismetSystemLibrary.Delay` 0.75)
  (`GameplayStatics.OpenLevel` "LVL_2_Main"))

(fn `OnRep_Event Instance`)

(fn `UserConstructionScript`)