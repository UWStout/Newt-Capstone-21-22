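; Pressure plate interactable that spawns a pushable box at a target reference's location when pressed.
; Trigger overlap swaps the plate material and plays the Push timeline, which moves the plate vertically.
; When the timeline finishes with the plate still pressed, it spawns BP_Pushable_Final at a fixed rotation.
; End overlap restores the material, but the plate only reverses and resets once the trigger is empty.
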(event `self.Trigger.OnComponentBeginOverlap`
  (params (OverlappedComponent :type "PrimitiveComponent Object Reference") (OtherActor :type "Actor Object Reference") (OtherComp :type "PrimitiveComponent Object Reference") (OtherBodyIndex :type Integer) (bFromSweep :type Boolean) (SweepResult :type "HitResult Structure (by ref)"))
  (`PrimitiveComponent.SetMaterial` (`self.Plate`) 0 "/Game/Art_Assets/Materials/Materials/M_ROCK_PressurePressed.M_ROCK_PressurePressed")
  (`KismetSystemLibrary.PrintString` "On")
  (if (not (`self.Pressed`))
    (set `self.Pressed` true)
    (bind (_direction _push) (`Timeline|Push` :!label _label)
      (:`Update`
        (`SceneComponent.K2_SetRelativeLocation` (`self.Plate`) (`KismetMathLibrary.MakeVector` 0.0 0.0 _push) false false))
      (:`Finished`
        (if (`self.Pressed`)
          (`|SpawnActorFromClass` :`Class` "/Game/Interactables/BP_Pushable_Final.BP_Pushable_Final_C" :`SpawnTransform` (`KismetMathLibrary.MakeTransform` (`self.K2_GetActorLocation` (`self.TargetReference`)) (struct :`Yaw` -40.0)) :`CollisionHandlingOverride` "Undefined" :`TransformScaleMethod` "OverrideRootScale" :`Instigator` null)
          (`KismetSystemLibrary.Delay` 5.0))))))

(event `self.Trigger.OnComponentEndOverlap`
  (params (OverlappedComponent :type "PrimitiveComponent Object Reference") (OtherActor :type "Actor Object Reference") (OtherComp :type "PrimitiveComponent Object Reference") (OtherBodyIndex :type Integer))
  (`PrimitiveComponent.SetMaterial` (`self.Plate`) 0 "/Game/Art_Assets/Materials/Materials/M_ROCK_Pressure.M_ROCK_Pressure")
  (`KismetSystemLibrary.PrintString` "Off")
  (if (not (`KismetArrayLibrary.Array_IsValidIndex` (`PrimitiveComponent.GetOverlappingActors` (`self.Trigger`) null)))
    (set `self.Pressed` false)
    (goto _label :!via `Reverse`)))

(fn `UserConstructionScript`)