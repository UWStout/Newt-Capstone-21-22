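; Ruins puzzle door that opens once Carry_Statue actors rest on both of its pedestals.
; Either trigger snaps an overlapping statue onto its pedestal, or the other if already filled, disabling physics and playing force feedback.
; With both filled, a timeline moves the door along Z, with sound and prompt cleanup.
; Elena's overlap with the actor toggles custom-depth pedestal highlights and prompt widgets chosen by whether she is carrying.
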(event `self.Trigger1.OnComponentBeginOverlap`
  (params (OverlappedComponent :type "PrimitiveComponent Object Reference") (OtherActor :type "Actor Object Reference") (OtherComp :type "PrimitiveComponent Object Reference") (OtherBodyIndex :type Integer) (bFromSweep :type Boolean) (SweepResult :type "HitResult Structure (by ref)"))
  (bind _alpha_v2_pasted__doorback (`self.Alpha_V2_pasted__doorBack`))
  (bind _pedestal_2 (`self.Pedestal_2`))
  (bind _output (`|ConvertAsset` (`self.UIControllerRef`)))
  ;[1 1 1] if this pedestal is already done, put it on the other
  (if (`self.LeftDone`)
    ;[1 1 1] Right Door Statue Mechanic
    (set `self.inRange` true :!label _label)
    (bind _ascarry_statue (cast `/Game/Interactables/Carry_Statue` (stale `self.Trigger2.OnComponentBeginOverlap` OtherActor)))
    (set `self.StatueRef` _ascarry_statue)
    (`self.K2_SetActorRotation` :`self` (stale `self.Trigger2.OnComponentBeginOverlap` OtherActor))
    (`self.K2_SetActorLocation` (stale `self.Trigger2.OnComponentBeginOverlap` OtherActor) (+ (`SceneComponent.K2_GetComponentLocation` (`self.Pedestal_2`)) (-70.0 -30.0 195.0)) false true)
    (bind _object (`/Game/Interactables/Carry_Statue.Object` _ascarry_statue))
    (`PrimitiveComponent.SetSimulatePhysics` _object false)
    (`PlayerController.K2_ClientPlayForceFeedback` (`GameplayStatics.GetPlayerController` 0) "/Game/Characters/ForceFeedback/TransformFeedbackEffect.TransformFeedbackEffect" "None" false false false)
    (`PrimitiveComponent.SetCollisionResponseToChannel` _object "ECC_GameTraceChannel4" "ECR_Ignore")
    (set `self.RightDone` true)
    (`/Game/UI/UI_Conroller.CheckRemoveBoth` (`|ConvertAsset` (`self.UIControllerRef`)) (stale `self.ReceiveActorBeginOverlap` _returnvalue))
    (`/Game/Interactables/Carry_Statue.OnPedestal` (`self.StatueRef`))
    (else
      ;[1 1 1] Left Door Statue Mechanic
      (set `self.InRange` true :!label _label_2)
      (bind _ascarry_statue_2 (cast `/Game/Interactables/Carry_Statue` OtherActor))
      (set `self.StatueRef` _ascarry_statue_2)
      (`self.K2_SetActorRotation` :`self` OtherActor)
      (`self.K2_SetActorLocation` OtherActor (+ (`SceneComponent.K2_GetComponentLocation` (`self.Pedestal_1`)) (-75.0 -10.0 195.0)) false true)
      (bind _object_2 (`/Game/Interactables/Carry_Statue.Object` _ascarry_statue_2))
      (`PrimitiveComponent.SetSimulatePhysics` _object_2 false)
      (`PlayerController.K2_ClientPlayForceFeedback` (`GameplayStatics.GetPlayerController` 0) "/Game/Characters/ForceFeedback/TransformFeedbackEffect.TransformFeedbackEffect" "None" false false false)
      (`PrimitiveComponent.SetCollisionResponseToChannel` _object_2 "ECC_GameTraceChannel4" "ECR_Ignore")
      (set `self.LeftDone` true)
      (`/Game/UI/UI_Conroller.CheckRemoveBoth` (`|ConvertAsset` (`self.UIControllerRef`)) (stale `self.ReceiveActorBeginOverlap` _returnvalue))
      (`/Game/Interactables/Carry_Statue.OnPedestal` (`self.StatueRef`))))
  ;[1 1 1] When both statues are on their pedestals, the door will open
  (if (and (`self.LeftDone`) (`self.RightDone`))
    (bind (_direction _newtrack_0) (`Timeline|Timeline_0`)
      (:`Update`
        (`SceneComponent.K2_SetRelativeLocation` _alpha_v2_pasted__doorback (`KismetMathLibrary.MakeVector` 0.0 0.0 _newtrack_0) false true)
        (`/Engine/EditorBlueprintResources/StandardMacros.DoOnce` false
          (:`Completed`
            (`FMODBlueprintStatics.PlayEventAttached` "/Game/FMOD/Events/game/02_ruins/stone_door_opening_ruins.stone_door_opening_ruins" _alpha_v2_pasted__doorback "None" (0.0 0.0 0.0) "KeepRelativeOffset")
            ;[1 1 1] remove all ui when complete
            (`/Game/UI/UI_Conroller.CheckRemoveBoth` _output (stale `self.ReceiveActorBeginOverlap` _returnvalue))
            (`/Game/UI/UI_Conroller.CheckRemoveBoth` _output (stale `self.ReceiveActorBeginOverlap` _returnvalue_2))
            ;[1 1 1] remove all highlight on complete
            (`PrimitiveComponent.SetRenderCustomDepth` _pedestal_2 false)
            (`PrimitiveComponent.SetRenderCustomDepth` (`self.Pedestal_1`) false)
            (`PrimitiveComponent.SetCustomDepthStencilValue` _pedestal_2 0)
            (`PrimitiveComponent.SetCustomDepthStencilValue` (`self.Pedestal_1`) 0)
            (`/Game/Interactables/Carry_Statue.OnPedestal` (`self.StatueRef`))))))))

(event `self.Trigger1.OnComponentEndOverlap`
  (params (OverlappedComponent :type "PrimitiveComponent Object Reference") (OtherActor :type "Actor Object Reference") (OtherComp :type "PrimitiveComponent Object Reference") (OtherBodyIndex :type Integer))
  ;[1 1 1] Left Door Statue Mechanic
  (set `self.InRange` false))

(event `self.Trigger2.OnComponentBeginOverlap`
  (params (OverlappedComponent :type "PrimitiveComponent Object Reference") (OtherActor :type "Actor Object Reference") (OtherComp :type "PrimitiveComponent Object Reference") (OtherBodyIndex :type Integer) (bFromSweep :type Boolean) (SweepResult :type "HitResult Structure (by ref)"))
  ;[1 1 1] if this pedestal is already done, put it on the other
  (if (`self.RightDone`)
    (goto _label_2)
    (else
      (goto _label))))

(event `self.Trigger2.OnComponentEndOverlap`
  (params (OverlappedComponent :type "PrimitiveComponent Object Reference") (OtherActor :type "Actor Object Reference") (OtherComp :type "PrimitiveComponent Object Reference") (OtherBodyIndex :type Integer))
  ;[1 1 1] Right Door Statue Mechanic
  (set `self.inRange` false))

(event `self.ReceiveActorBeginOverlap`
  (params (OtherActor :type "Actor Object Reference"))
  (bind _pedestal_2 (`self.Pedestal_2`))
  ;[1 1 1] Highlight/ Dectect correct actor to display message and display highlight
  (bind _aselena (cast `/Game/Characters/Elena/Elena` OtherActor))
  (`AddComponent|NODE_AddHighlighter-12` :`self` _aselena)
  (`PrimitiveComponent.SetRenderCustomDepth` _pedestal_2 true)
  (`PrimitiveComponent.SetRenderCustomDepth` (`self.Pedestal_1`) true)
  (`PrimitiveComponent.SetCustomDepthStencilValue` _pedestal_2 4)
  (`PrimitiveComponent.SetCustomDepthStencilValue` (`self.Pedestal_1`) 4)
  (bind _aselena_2 (cast `/Game/Characters/Elena/Elena` (`GameplayStatics.GetPlayerCharacter` 0)))
  (set `self.ElenaRef` _aselena_2)
  (if (`/Game/Characters/Elena/Elena.IsCarrying` (`self.ElenaRef`))
    (bind _returnvalue (`|CreateWidget` "/Game/UI/Interaction_Buttons/Interact_Pedestal.Interact_Pedestal_C"))
    (`/Game/UI/UI_Conroller.DrawElena` (`|ConvertAsset` (`self.UIControllerRef`)) _returnvalue)
    (elif (not (and (`self.LeftDone`) (`self.RightDone`)))
      (bind _returnvalue_2 (`|CreateWidget` "/Game/UI/Interaction_Buttons/Interact_TwoPedestals.Interact_TwoPedestals_C"))
      (`/Game/UI/UI_Conroller.DrawElena` (`|ConvertAsset` (`self.UIControllerRef`)) _returnvalue_2))))

(event `self.ReceiveActorEndOverlap`
  (params (OtherActor :type "Actor Object Reference"))
  (bind _pedestal_2 (`self.Pedestal_2`))
  (bind _output (`|ConvertAsset` (`self.UIControllerRef`)))
  ;[1 1 1] Highlight/ Dectect correct actor to display message and display highlight
  (bind _aselena (cast `/Game/Characters/Elena/Elena` OtherActor))
  (`AddComponent|NODE_AddHighlighter-13` :`self` _aselena)
  (`PrimitiveComponent.SetRenderCustomDepth` _pedestal_2 false)
  (`PrimitiveComponent.SetRenderCustomDepth` (`self.Pedestal_1`) false)
  (`PrimitiveComponent.SetCustomDepthStencilValue` _pedestal_2 0)
  (`PrimitiveComponent.SetCustomDepthStencilValue` (`self.Pedestal_1`) 0)
  (`/Game/UI/UI_Conroller.CheckRemoveBoth` _output (stale `self.ReceiveActorBeginOverlap` _returnvalue))
  (`/Game/UI/UI_Conroller.CheckRemoveBoth` _output (stale `self.ReceiveActorBeginOverlap` _returnvalue_2)))

(fn `UserConstructionScript`)