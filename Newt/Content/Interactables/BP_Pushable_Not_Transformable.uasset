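; Pushable object that Elena can push, showing an outline and push/pull prompt while she overlaps it.
; Designer-set PushTransforms define the push sides, previewed as arrows by the construction script.
; On Push, it picks the nearest side within the character's PushRange and validates standing room, walkable floor and obstructions with traces.
; It then teleports the character there, nudges Newt's mesh upward and starts PushComponentNotTransformable's push, printing any failure reason.
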(event `self.ReceiveActorBeginOverlap`
  (params (OtherActor :type "Actor Object Reference"))
  (bind _output (`|ConvertAsset` (`self.UIControllerRef`)))
  ;[1 1 1] Highlight/ Dectect correct Elena to display message and display highlight
  (bind _aselena (cast `/Game/Characters/Elena/Elena` OtherActor))
  (`AddComponent|NODE_AddHighlighter-0` :`self` _aselena)
  (`PrimitiveComponent.SetRenderCustomDepth` (`self.StaticMesh`) true)
  (`PrimitiveComponent.SetCustomDepthStencilValue` null 1)
  (`PrimitiveComponent.SetCustomDepthStencilValue` (`self.StaticMesh`) 1)
  ;[1 1 1] Pushing/Pulling UI
  (`/Engine/EditorBlueprintResources/StandardMacros.DoOnce` false :!label _label
    (:`Completed`
      (`/Game/UI/UI_Conroller.RemoveBoth` (`|ConvertAsset` (`self.UIControllerRef`)))
      (bind _returnvalue (`|CreateWidget` "/Game/UI/Interaction_Buttons/Interact_PushPull.Interact_PushPull_C"))
      (`/Game/UI/Interaction_Buttons/Interact_PushPull.Swap Text` _returnvalue _output)
      (bind _output_get (set `/Game/UI/UI_Conroller.UI_Prompt_Elena` _returnvalue _output))
      (`/Game/UI/UI_Conroller.DrawElena` (`|ConvertAsset` (`self.UIControllerRef`)) _output_get))))

(event `self.ReceiveBeginPlay`
  ;[1 1 1] Get UI Contoller ref if not manually set
  (bind _returnvalue (`GameplayStatics.GetActorOfClass` "/Game/Characters/Newt/Newt.Newt_C"))
  (set `self.Newt` _returnvalue)
  (if (not (`KismetSystemLibrary.IsValid` (`|ConvertAsset` (`self.UIControllerRef`))))
    (bind _returnvalue_2 (`GameplayStatics.GetActorOfClass` "/Game/UI/UI_Conroller.UI_Conroller_C"))
    (set `self.UIControllerRef` (`|ConvertAsset` _returnvalue_2))))

(event `self.ReceiveActorEndOverlap`
  (params (OtherActor :type "Actor Object Reference"))
  ;[1 1 1] Highlight/ Dectect correct Elena to display message and display highlight
  (bind _aselena (cast `/Game/Characters/Elena/Elena` OtherActor))
  (`AddComponent|NODE_AddHighlighter-1` :`self` _aselena)
  (`PrimitiveComponent.SetRenderCustomDepth` (`self.StaticMesh`) false)
  (`PrimitiveComponent.SetCustomDepthStencilValue` null 0)
  (`PrimitiveComponent.SetCustomDepthStencilValue` (`self.StaticMesh`) 0)
  ;[1 1 1] Pushing/Pulling UI
  (`/Game/UI/UI_Conroller.CheckRemoveBoth` (`|ConvertAsset` (`self.UIControllerRef`)) (stale `self.ReceiveActorBeginOverlap` _returnvalue) :!label _label_2)
  (goto _label :!via `Reset`))

(event `InputAction|Push`
  (params (Key :type "Key Structure"))
  ;[1 1 1] Pushing/Pulling UI
  (:`Released`
    (goto _label_2)))

(event `/Game/Interfaces/Pushable.Push`
  (params (Elena :type "/Game/Characters/Elena/Elena Object Reference"))
  ;[1 1 1] Start pushing
  (`self.HandleInteraction` Elena))

(fn `FindClosestPushTransformIndex`
  (params (CharacterLocation :type "Vector2D Structure") (PushRange :type "Float (double-precision)"))
  (returns (BestIndex :type Integer))
  (locals (CurrentTransformIndex :type Integer) (CurrentDistanceSquared :type "Float (double-precision)" :default 0.0) (ClosestTransformIndex :type Integer :default -1) (ClosestDistanceSquared :type "Float (double-precision)"))
  ;[1 1 1] Find the closest index to the character's current position and return it
  (for (_array_element _array_index) (`self.PushTransforms`)
    (set `local.CurrentTransformIndex` _array_index)
    (bind _output_get (set `local.CurrentDistanceSquared` (`KismetMathLibrary.DistanceSquared2D` (`KismetMathLibrary.Conv_VectorToVector2D` (`KismetMathLibrary.TransformLocation` (`self.GetTransform`) (.location _array_element))) (`local.CharacterLocation`))))
    (if (< _output_get (`KismetMathLibrary.Square` (`local.PushRange`)))
      (if (or (< (`local.CurrentDistanceSquared`) (`local.ClosestDistanceSquared`)) (< (`local.ClosestTransformIndex`) 0))
        (set `local.ClosestTransformIndex` (`local.CurrentTransformIndex`))
        (set `local.ClosestDistanceSquared` (`local.CurrentDistanceSquared`)))))
  (return (`local.ClosestTransformIndex`)))

(fn `HandleInteraction`
  (params (Character :type "/Game/Characters/Elena/Elena Object Reference"))
  (locals (PushComponent :type "/Game/TestLevels/Anton/Blueprints/Pushable/PushComponentNotTransformable Object Reference") (CharacterNewTransform :type "Transform Structure"))
  (bind _characternewtransform_location (`KismetMathLibrary.BreakTransform` (`local.CharacterNewTransform`)))
  (bind _characternewtransform_location_2 (`KismetMathLibrary.BreakTransform` (`local.CharacterNewTransform`)))
  (bind _mesh (`Character.Mesh` (`self.Newt`)))
  (bind _capsulecomponent (`Character.CapsuleComponent` (`local.Character`)))
  ;[1 1 1] Check if the character is valid
  (`/Engine/EditorBlueprintResources/StandardMacros.IsValid` Character
    (:`Is Valid`
      (bind _output_get (set `local.PushComponent` (`self.GetComponentByClass` Character "/Game/TestLevels/Anton/Blueprints/Pushable/PushComponentNotTransformable.PushComponentNotTransformable_C")))
      (`/Engine/EditorBlueprintResources/StandardMacros.IsValid` _output_get
        (:`Is Valid`
          ;[1 1 1] Detect the side to push
          (bind _bestindex (`self.FindClosestPushTransformIndex` (`KismetMathLibrary.Conv_VectorToVector2D` (`self.K2_GetActorLocation` (`local.Character`))) (`/Game/TestLevels/Anton/Blueprints/Pushable/PushComponentNotTransformable.PushRange` (`local.PushComponent`))))
          (if (>= _bestindex 0)
            (bind (_returnvalue_location _returnvalue_rotation) (`KismetMathLibrary.BreakTransform` (`KismetMathLibrary.ComposeTransforms` (`|GetArrayItem` (`self.PushTransforms`) _bestindex) (`self.GetTransform`))))
            (set `local.CharacterNewTransform` (`KismetMathLibrary.MakeTransform` (+ _returnvalue_location (`KismetMathLibrary.MakeVector` 0.0 0.0 (`CapsuleComponent.GetScaledCapsuleHalfHeight` (`Character.CapsuleComponent` (`local.Character`))))) _returnvalue_rotation))
            (bind _outhit (`KismetSystemLibrary.CapsuleTraceSingle` :`Start` (+ _characternewtransform_location_2 (0.0 0.0 70.0)) :`End` (- _characternewtransform_location_2 (0.0 0.0 100.0)) :`Radius` (`CapsuleComponent.GetScaledCapsuleRadius` _capsulecomponent) :`HalfHeight` (`CapsuleComponent.GetScaledCapsuleHalfHeight` _capsulecomponent) :`TraceChannel` "TraceTypeQuery1" :`DrawTime` 2.0))
            (bind (_bblockinghit _binitialoverlap _time _distance _location _impactpoint _normal _impactnormal) (`GameplayStatics.BreakHitResult` _outhit))
            ;[1 1 1] Check if the floor is walkable
            (if (not _binitialoverlap)
              (if (< (`CharacterMovementComponent.K2_GetWalkableFloorZ` (`Character.CharacterMovement` (`local.Character`))) (.z _impactnormal))
                ;[1 1 1] Check if there is an obstacle between the character and a pushable object
                (bind (_outhit_2 _returnvalue) (`KismetSystemLibrary.LineTraceSingle` (`self.K2_GetActorLocation`) _characternewtransform_location "TraceTypeQuery1" false (`|MakeArray` (`local.Character`) :!type "Actor Object Reference") "None" true (struct :`R` 1.0 :`A` 1.0) (struct :`G` 1.0 :`A` 1.0) 2.0))
                (if (not _returnvalue)
                  ;[1 1 1] Set character's transform and start pushing
                  (`self.K2_SetActorTransform` (`local.Character`) (`local.CharacterNewTransform`) false true)
                  (`SceneComponent.K2_SetWorldLocation` _mesh (+ (`SceneComponent.K2_GetComponentLocation` _mesh) (0.0 0.0 3.5)) false false)
                  (`/Game/TestLevels/Anton/Blueprints/Pushable/PushComponentNotTransformable.BeginPush` (`local.PushComponent`) self)
                  (else
                    (`self.PushFailedInfo` "Wall in between character and an object")))
                (else
                  (`self.PushFailedInfo` "Floor not walkable")))
              (else
                (`self.PushFailedInfo` "No room to stand")))
            (else
              (`self.PushFailedInfo` "No push transform found"))))
        (:`Is Not Valid`
          (`self.PushFailedInfo` "Character does not have push component"))))
    (:`Is Not Valid`
      (`self.PushFailedInfo` "Character is invalid"))))

(fn `Interact`
  (returns (Interacted :type Boolean))
  (return false))

(fn `UserConstructionScript`
  ;[1 1 1] Add arrows to indicate the pushing sides
  (for _array_element (`self.PushTransforms`)
    (`AddComponent|NODE_AddArrowComponent-0` :`RelativeTransform` _array_element)))