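; Pressure plate puzzle actor that raises three platforms while pressed and lowers them after it is released.
; Trigger overlaps swap the plate material and drive the Push timeline, whose finish after release starts a delay before setting Lower.
; Tick reads Pressed and Lower, calling MovePlatform to lerp each platform's world Z toward hard-coded heights.
; Older timeline-based platform movement remains disconnected, and Raise is set but never read.
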(event `self.ReceiveTick`
  (params (DeltaSeconds :type "Float (single-precision)"))
  (bind _platform2 (`self.Platform2`))
  (bind _platform3 (`self.Platform3`))
  (if (`self.Pressed`)
    ;[1 1 1] Move platform 1
    (`self.MovePlatform` (`self.Platform1`) -1091.0)
    ;[1 1 1] move platform 2
    (`self.MovePlatform` _platform2 -1205.0)
    ;[1 1 1] move platform 3
    (`self.MovePlatform` _platform3 -1205.0)
    (elif (`self.Lower`)
      (`self.MovePlatform` (`self.Platform1`) -1597.0)
      (`self.MovePlatform` _platform2 -1676.0)
      (`self.MovePlatform` _platform3 -1692.0))))

(event `self.Trigger.OnComponentBeginOverlap`
  (params (OverlappedComponent :type "PrimitiveComponent Object Reference") (OtherActor :type "Actor Object Reference") (OtherComp :type "PrimitiveComponent Object Reference") (OtherBodyIndex :type Integer) (bFromSweep :type Boolean) (SweepResult :type "HitResult Structure (by ref)"))
  (`PrimitiveComponent.SetMaterial` (`self.Plate`) 0 "/Game/Art_Assets/Materials/Materials/MI_ROCK_PressurePressed.MI_ROCK_PressurePressed")
  (if (not (`self.Pressed`))
    (set `self.Pressed` true)
    (bind (_direction _push) (`Timeline|Push` :!label _label)
      (:`Update`
        (`SceneComponent.K2_SetRelativeLocation` (`self.Plate`) (`KismetMathLibrary.MakeVector` 0.0 0.0 _push) false false))
      (:`Finished`
        (if (`self.Pressed`)
          (set `self.Raise` true)
          (set `self.Lower` false)
          (else
            (`KismetSystemLibrary.Delay` 7.0)
            (set `self.Lower` true)))))))

(event `self.Trigger.OnComponentEndOverlap`
  (params (OverlappedComponent :type "PrimitiveComponent Object Reference") (OtherActor :type "Actor Object Reference") (OtherComp :type "PrimitiveComponent Object Reference") (OtherBodyIndex :type Integer))
  (`PrimitiveComponent.SetMaterial` (`self.Plate`) 0 "/Game/Art_Assets/Materials/Materials/MI_ROCK_Pressure.MI_ROCK_Pressure")
  (if (not (`KismetArrayLibrary.Array_IsValidIndex` (`PrimitiveComponent.GetOverlappingActors` (`self.Trigger`) null)))
    (set `self.Pressed` false)
    (goto _label :!via `Reverse`)))

(fn `MovePlatform`
  (params (Platform :type "StaticMeshActor Object Reference") (`Z Target` :type "Float (double-precision)"))
  (bind _rootcomponent (`Actor.RootComponent` Platform))
  (bind (_returnvalue_x _returnvalue_y _returnvalue_z) (`KismetMathLibrary.BreakVector` (`SceneComponent.K2_GetComponentLocation` _rootcomponent)))
  (bind (_returnvalue_x_2 _returnvalue_y_2 _returnvalue_z_2) (`KismetMathLibrary.BreakVector` (`SceneComponent.K2_GetComponentLocation` _rootcomponent)))
  ;[1 1 1] Raise Platform
  (if (not (< (`KismetMathLibrary.Abs` (- `Z Target` _returnvalue_z)) 10.0))
    (`SceneComponent.K2_SetWorldLocation` _rootcomponent (`KismetMathLibrary.MakeVector` _returnvalue_x_2 _returnvalue_y_2 (`KismetMathLibrary.Lerp` _returnvalue_z_2 `Z Target` (`self.Step`))) false false)))

(fn `UserConstructionScript`)