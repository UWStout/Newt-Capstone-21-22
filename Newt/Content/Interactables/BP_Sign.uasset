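; BP_Sign is an interactable sign that shows a separate UI widget to each of the two characters, Elena and Newt, on overlap.
; Entering removes that character's UI prompt, creates its configured sign widget and passes it to the UI controller to draw.
; Leaving asks the controller to check and remove that widget.
; The controller reference is found in the level at BeginPlay if not set manually.
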(event `self.ReceiveBeginPlay`
  ;[1 1 1] Get UI Contoller ref if not manually set
  (if (not (`KismetSystemLibrary.IsValid` (`|ConvertAsset` (`self.UIControllerRef`))))
    (bind _returnvalue (`GameplayStatics.GetActorOfClass` "/Game/UI/UI_Conroller.UI_Conroller_C"))
    (set `self.UIControllerRef` (`|ConvertAsset` _returnvalue))))

(event `self.ReceiveActorBeginOverlap`
  (params (OtherActor :type "Actor Object Reference"))
  (bind _newtsignwiget (`self.NewtSignWiget`))
  (bind _elenasignwiget (`self.ElenaSignWiget`))
  ;[1 1 1] Event ActorBeginOverlap - Other Actor -> Object for casts
  ;[1 1 1] this is bryces code
  (cast `/Game/Characters/Elena/Elena` OtherActor
    (:`then`
      (`Widget.RemoveFromParent` (`/Game/UI/UI_Conroller.UI_Prompt_Elena` (`|ConvertAsset` (`self.UIControllerRef`))))
      (if (`KismetSystemLibrary.IsValidClass` _elenasignwiget)
        (bind _returnvalue (`|CreateWidget` _elenasignwiget))
        (bind _output_get (set `self.ElenaSignUI` _returnvalue))
        (`/Game/UI/UI_Conroller.DrawElena` (`|ConvertAsset` (`self.UIControllerRef`)) _output_get)))
    (:`CastFailed`
      (cast `/Game/Characters/Newt/Newt` OtherActor)
      (`Widget.RemoveFromParent` (`/Game/UI/UI_Conroller.UI_Prompt_Newt` (`|ConvertAsset` (`self.UIControllerRef`))))
      (if (`KismetSystemLibrary.IsValidClass` _newtsignwiget)
        (bind _returnvalue_2 (`|CreateWidget` _newtsignwiget))
        (bind _output_get_2 (set `self.NewtSignUI` _returnvalue_2))
        (`/Game/UI/UI_Conroller.DrawNewt` (`|ConvertAsset` (`self.UIControllerRef`)) _output_get_2)))))

(event `self.ReceiveActorEndOverlap`
  (params (OtherActor :type "Actor Object Reference"))
  (cast `/Game/Characters/Elena/Elena` OtherActor
    (:`then`
      (`/Game/UI/UI_Conroller.CheckRemoveElena` (`|ConvertAsset` (`self.UIControllerRef`)) (`self.ElenaSignUI`)))
    (:`CastFailed`
      (cast `/Game/Characters/Newt/Newt` OtherActor)
      (`/Game/UI/UI_Conroller.CheckRemoveNewt` (`|ConvertAsset` (`self.UIControllerRef`)) (`self.NewtSignUI`)))))

(fn `UserConstructionScript`)