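; Test Blueprint in a developer test level that holds an unfinished movement input graph with no working behavior.
; MoveForward and MoveRight axis events check a Transformed flag and a nonzero axis value, then do nothing.
; Disconnected leftovers of the original movement code, including yaw-only direction math and AddMovementInput calls, never run.
; BeginPlay, Tick and the construction script are empty.
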(event `InputAxis|MoveForward` :overrideparent false
  (params (AxisValue :type "Float (single-precision)"))
  ;[1 1 1] Movement input,Both Mix
  (if (`self.Transformed`)
    (if (!= AxisValue 0.0)
      _)))

(event `InputAxis|MoveRight` :overrideparent false
  (params (AxisValue :type "Float (single-precision)"))
  ;[1 1 1] Movement input,Both Mix
  (if (`self.Transformed`)
    (if (!= AxisValue 0.0)
      _)))

(fn `UserConstructionScript`)