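; Actor component on Elena that lets her push and pull pushable objects, with controller rumble.
; BeginPush attaches her to the object, constrains movement to a plane and enables Tick; EndPush reverses this, restores the object's physics and nudges Newt's mesh down.
; While she is controlled, Tick polls forward/back input and moves the object along her facing, setting a direction value.
; Pushing uses swept offsets; pulling also capsule-traces behind her for obstacles.
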(event `self.ReceiveBeginPlay`
  ;[1 1 1] Set variables
  (`self.SetComponentTickEnabled` false)
  (bind _returnvalue (`GameplayStatics.GetActorOfClass` "/Game/Characters/Elena/Elena.Elena_C"))
  (set `self.Elena` _returnvalue)
  (bind _returnvalue_2 (`GameplayStatics.GetActorOfClass` "/Game/Characters/Newt/Newt.Newt_C"))
  (set `self.Newt` _returnvalue_2)
  (bind _returnvalue_3 (`GameplayStatics.GetActorOfClass` "/Game/Interactables/BP_Pushable_Not_Transformable.BP_Pushable_Not_Transformable_C"))
  (set `self.PushableNotTransformable` _returnvalue_3))

(event `self.ReceiveTick`
  (params (DeltaSeconds :type "Float (single-precision)"))
  ;[1 1 1] Push forward if W key is pressed
  (if (or (`PlayerController.IsInputKeyDown` (`GameplayStatics.GetPlayerController` 0) "Gamepad_LeftStick_Up") (`PlayerController.IsInputKeyDown` (`GameplayStatics.GetPlayerController` 0) "W"))
    (`self.PushForward` DeltaSeconds)
    (if (`/Game/Characters/Elena/Elena.Controlled` (`self.Elena`))
      (`PlayerController.K2_ClientPlayForceFeedback` (`GameplayStatics.GetPlayerController` 0) "/Game/Characters/ForceFeedback/PushingFeedbackEffect.PushingFeedbackEffect" "None" false false false))
    (else
      ;[1 1 1] Pull backwards if S key is pressed
      (if (or (`PlayerController.IsInputKeyDown` (`GameplayStatics.GetPlayerController` 0) "Gamepad_LeftStick_Down") (`PlayerController.IsInputKeyDown` (`GameplayStatics.GetPlayerController` 0) "S"))
        (`self.PushBackwards` DeltaSeconds)
        (if (`/Game/Characters/Elena/Elena.Controlled` (`self.Elena`))
          (`PlayerController.K2_ClientPlayForceFeedback` (`GameplayStatics.GetPlayerController` 0) "/Game/Characters/ForceFeedback/PushingFeedbackEffect.PushingFeedbackEffect" "None" false false false))
        (else
          (set `self.PushingDirection` 0)
          (`PlayerController.ClientStopForceFeedback` (`GameplayStatics.GetPlayerController` 0) "/Game/Characters/ForceFeedback/PushingFeedbackEffect.PushingFeedbackEffect" "None"))))))

(fn `BeginPush`
  (params (Pushable :type "/Game/Interactables/BP_Pushable_Final Object Reference"))
  (locals (OwningCharacter :type "Character Object Reference"))
  (bind _owningcharacter (`local.OwningCharacter`))
  (bind _charactermovement (`Character.CharacterMovement` _owningcharacter))
  ;[1 1 1] Set variables
  (if (not (`KismetSystemLibrary.IsValid` (`self.CurrentPushable`)))
    (bind _aselena (cast `/Game/Characters/Elena/Elena` (`self.GetOwner`)))
    (set `local.OwningCharacter` _aselena)
    (bind _output_get (set `self.CurrentPushable` (`local.Pushable`)))
    ;[1 1 1] Set Elena to the pushing state
    (`Actor.K2_AttachToActor` (`local.OwningCharacter`) _output_get "None" "KeepWorld" "KeepWorld" "KeepWorld" true)
    (`MovementComponent.SetPlaneConstraintEnabled` _charactermovement true)
    (`MovementComponent.SetPlaneConstraintNormal` _charactermovement (`Actor.GetActorRightVector` _owningcharacter))
    (set `CharacterMovementComponent.bOrientRotationToMovement` false _charactermovement)
    (`self.SetComponentTickEnabled` true)))

(fn `EndPush`
  (locals (OwningCharacter :type "Character Object Reference"))
  (bind _charactermovement (`Character.CharacterMovement` (`local.OwningCharacter`)))
  (bind _mesh (`Character.Mesh` (`self.Newt`)))
  ;[1 1 1] Set variables
  (`self.CurrentPushable`
    (:`then`
      (bind _ascharacter (cast `Character` (`self.GetOwner`)))
      (bind _output_get (set `local.OwningCharacter` _ascharacter))
      ;[1 1 1] Take Elena out of the pushing state
      (`Actor.K2_DetachFromActor` _output_get "KeepWorld" "KeepWorld" "KeepWorld")
      (`MovementComponent.SetPlaneConstraintEnabled` _charactermovement false)
      (set `CharacterMovementComponent.bOrientRotationToMovement` true _charactermovement)
      (`PrimitiveComponent.SetSimulatePhysics` (`/Game/Interactables/BP_Pushable_Final.StaticMesh` (`self.CurrentPushable`)) true)
      (`SceneComponent.K2_SetWorldLocation` _mesh (- (`SceneComponent.K2_GetComponentLocation` _mesh) (0.0 0.0 3.5)) false false)
      (`PlayerController.ClientStopForceFeedback` (`GameplayStatics.GetPlayerController` 0) "/Game/Characters/ForceFeedback/PushingFeedbackEffect.PushingFeedbackEffect" "None")
      (`self.SetComponentTickEnabled` false)
      (set `self.CurrentPushable` null)
      (set `self.PushingDirection` 0))
    (:`else`)))

(fn `IsPushingObject`
  (returns (ReturnValue :type Boolean))
  (return (`KismetSystemLibrary.IsValid` (`self.CurrentPushable`))))

(fn `PushBackwards`
  (params (DeltaSeconds :type "Float (double-precision)"))
  (bind _returnvalue (`Actor.K2_GetActorLocation` (`self.GetOwner`)))
  (bind _returnvalue_2 (* (* (`Actor.GetActorForwardVector` (`self.GetOwner`)) -1) (* DeltaSeconds (`self.PushSpeed`))))
  (if (`/Game/Characters/Elena/Elena.Controlled` (`self.Elena`))
    (set `self.PushingDirection` -1)
    (bind _currentpushable (`self.CurrentPushable`)
      (:`then`
        (bind (_outhit _returnvalue_3) (`KismetSystemLibrary.CapsuleTraceSingle` _returnvalue (+ _returnvalue (* _returnvalue_2 5.0)) 42.0 135.0 "TraceTypeQuery1"))
        (if (not _returnvalue_3)
          (`Actor.K2_AddActorWorldOffset` _currentpushable _returnvalue_2 true false)))
      (:`else`))))

(fn `PushForward`
  (params (DeltaSeconds :type "Float (double-precision)"))
  (if (`/Game/Characters/Elena/Elena.Controlled` (`self.Elena`))
    (set `self.PushingDirection` 1)
    (bind _currentpushable (`self.CurrentPushable`)
      (:`then`
        (`Actor.K2_AddActorWorldOffset` _currentpushable (* (`Actor.GetActorForwardVector` (`self.GetOwner`)) (* DeltaSeconds (`self.PushSpeed`))) true false))
      (:`else`))))